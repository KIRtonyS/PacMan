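; Two-way teleport gateway that moves the player between two gate components, Gate1 and Gate2.
; Overlapping either gate with an actor tagged Player disables collision on the other gate, then sets player character 0 to that gate's location.
; Disabling the destination's collision first guards against an instant bounce back.
; When a tagged actor's overlap with either gate ends, both gates regain query and physics collision after a short delay.
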(event `self.Gate1.OnComponentBeginOverlap`
  (params (OverlappedComponent :type "PrimitiveComponent Object Reference") (OtherActor :type "Actor Object Reference") (OtherComp :type "PrimitiveComponent Object Reference") (OtherBodyIndex :type Integer) (bFromSweep :type Boolean) (SweepResult :type "HitResult Structure (by ref)"))
  (if (`self.ActorHasTag` OtherActor "Player")
    (`PrimitiveComponent.SetCollisionEnabled` (`self.Gate2`) "NoCollision")
    (`self.K2_SetActorLocation` (`GameplayStatics.GetPlayerCharacter` 0) (`SceneComponent.K2_GetComponentLocation` (`self.Gate2`)) false false)))

(event `self.Gate2.OnComponentEndOverlap`
  (params (OverlappedComponent :type "PrimitiveComponent Object Reference") (OtherActor :type "Actor Object Reference") (OtherComp :type "PrimitiveComponent Object Reference") (OtherBodyIndex :type Integer))
  (if (`self.ActorHasTag` OtherActor "Player")
    (`KismetSystemLibrary.Delay` 1.0)
    (`PrimitiveComponent.SetCollisionEnabled` (`self.Gate2`) "QueryAndPhysics")
    (`PrimitiveComponent.SetCollisionEnabled` (`self.Gate1`) "QueryAndPhysics")))

(event `self.Gate1.OnComponentEndOverlap`
  (params (OverlappedComponent :type "PrimitiveComponent Object Reference") (OtherActor :type "Actor Object Reference") (OtherComp :type "PrimitiveComponent Object Reference") (OtherBodyIndex :type Integer))
  (if (`self.ActorHasTag` OtherActor "Player")
    (`KismetSystemLibrary.Delay` 1.0)
    (`PrimitiveComponent.SetCollisionEnabled` (`self.Gate1`) "QueryAndPhysics")
    (`PrimitiveComponent.SetCollisionEnabled` (`self.Gate2`) "QueryAndPhysics")))

(event `self.Gate2.OnComponentBeginOverlap`
  (params (OverlappedComponent :type "PrimitiveComponent Object Reference") (OtherActor :type "Actor Object Reference") (OtherComp :type "PrimitiveComponent Object Reference") (OtherBodyIndex :type Integer) (bFromSweep :type Boolean) (SweepResult :type "HitResult Structure (by ref)"))
  (if (`self.ActorHasTag` OtherActor "Player")
    (`PrimitiveComponent.SetCollisionEnabled` (`self.Gate1`) "NoCollision")
    (`self.K2_SetActorLocation` (`GameplayStatics.GetPlayerCharacter` 0) (`SceneComponent.K2_GetComponentLocation` (`self.Gate1`)) false false)))

(fn `UserConstructionScript`)